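; RobotSpectatorBP shows the state of robot parts in an on-screen arm status widget.
; On BeginPlay it creates a WBP_ArmStatus widget for player 0, adds it to the viewport and binds to RobotInteraction's OnPartStateChanged event.
; When that event fires with a valid part, it writes the part's state string to the widget, so the display updates by event rather than by polling.
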(event `self.ReceiveBeginPlay`
  ;[0.15 0.15 0.15 0.2812] Initialize UI and bind the interaction event
  (bind _returnvalue (`|CreateWidget` "/Game/Widgets/WBP_ArmStatus.WBP_ArmStatus_C" (`GameplayStatics.GetPlayerController` 0)))
  (bind _output_get (set `self.PartStatus` _returnvalue))
  (`UserWidget.AddToViewport` _returnvalue 0)
  (`UserWidget.AddToViewport` _output_get 0)
  (add `RobotInteractionComponent.OnPartStateChanged` (`self.RobotInteraction`) (delegate `OnPartStateChanged_Event`)))

(event `OnPartStateChanged_Event`
  (params (Part :type "AttachablePart Object Reference"))
  ;[0.15 0.15 0.15 0.2812] Initialize UI and bind the interaction event
  (if (`KismetSystemLibrary.IsValid` Part)
    (`/Game/Widgets/WBP_ArmStatus.SetText` (`self.PartStatus`) (`KismetTextLibrary.Conv_StringToText` (`AttachablePart.GetStateAsString` Part)))))

(fn `UserConstructionScript`)